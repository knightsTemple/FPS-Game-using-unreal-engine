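; BP_Hoshino is a character Blueprint that adds health-change feedback and an on-screen widget for the Hoshino character.
; On BeginPlay it binds its attribute component's health-changed event to a camera shake and creates a MinionWidget_BP attached to itself.
; The shake plays on player 0's camera manager for any health change, without checking the delta.
; A Parry action call through the action component exists but is unconnected.
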(event Custom|shake
  (params (InstigatorActor :type Actor%20Object%20Reference) (OwningComp :type S%20Attribute%20Component%20Object%20Reference) (NewHealth :type Float%20%28single-precision%29) (Delta :type Float%20%28single-precision%29))
  (Class|PlayerCameraManager|StartCameraShakefromSource (Game|GetPlayerCameraManager 0) "/Game/MyPerson/Actor/ShakeCamera.ShakeCamera_C" 0 6.0 "CameraLocal" "0, 0, 0"))

(event EventBeginPlay
  (EventDispatchers|BindEventtoOnHealthChanged (Variables|Default|GetAttributeComp) (delegate Custom|shake))
  (bind _returnvalue (UserInterface|CreateWidget "/Game/MyPerson/UI/MinionWidget_BP.MinionWidget_BP_C" 0 self))
  (UserInterface|Viewport|AddtoViewport _returnvalue 0))

(event Collision|EventActorBeginOverlap
  (params (OtherActor :type Actor%20Object%20Reference)))

(event EventTick
  (params (DeltaSeconds :type Float%20%28single-precision%29)))

(event Input|ActionEvents|InputActionParry
  (params (Key :type Key%20Structure :default "None")))

(fn ConstructionScript)