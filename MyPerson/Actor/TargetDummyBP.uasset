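; TargetDummyBP is a target dummy actor that shows damage pop-ups when hit and is destroyed when its health runs out.
; Its AttributeComp health-change event spawns a DamagePopUp_Widget attached to the dummy and records the dummy as HitActor on MY_GameInstance.
; The pop-up and HitActor update run on every health change, while destruction requires depleted health and a non-positive delta.
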(event OnHealthChanged(AttributeComp)
  (params (InstigatorActor :type Actor%20Object%20Reference) (OwningComp :type S%20Attribute%20Component%20Object%20Reference) (NewHealth :type Float%20%28single-precision%29) (Delta :type Float%20%28single-precision%29))
  (bind _returnvalue (UserInterface|CreateWidget "/Game/MyPerson/UI/DamagePopUp_Widget.DamagePopUp_Widget_C" 0 self))
  (UserInterface|Viewport|AddtoViewport _returnvalue 0)
  (Variables|/Game/MyPerson/Actor/MY_GameInstance.MY_GameInstance_C|SetHitActor (.AsMY%20Game%20Instance (Utilities|Casting|CastToMY_GameInstance (Game|GetGameInstance))) self)
  (if (and (<= NewHealth 0.0) (<= Delta 0.0))
    (Actor|DestroyActor)))

(event EventBeginPlay)

(event Collision|EventActorBeginOverlap
  (params (OtherActor :type Actor%20Object%20Reference)))

(event EventTick
  (params (DeltaSeconds :type Float%20%28single-precision%29)))

(fn ConstructionScript)